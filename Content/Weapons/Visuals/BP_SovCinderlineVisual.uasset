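; Visual Blueprint for the SovCinderline weapon, supplying its meshes and melee collision.
; The construction script registers iron sights, with a separate local mesh, as the default attachment for the Narrative scope slot.
; GetCollidingPrimitives returns the MeleeCollider as the weapon's only colliding primitive.
; The event graph holds only disabled placeholder events, so no runtime logic runs there.
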(fn `GetCollidingPrimitives`
  (returns (ReturnValue :type "Array of PrimitiveComponent Object Reference"))
  (return (`|MakeArray` (`self.MeleeCollider`) :!type "PrimitiveComponent Object Reference")))

(fn `UserConstructionScript`
  (`parent.UserConstructionScript`)
  (`self.RegisterDefaultAttachment` (`BlueprintGameplayTagLibrary.MakeLiteralGameplayTag` (struct :`TagName` "Narrative.Equipment.Weapon.AttachSlot.Scope")) (`self.IronSights`) (`self.LocalIronSights`)))