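; Camera director for the Sov player character that picks and parameterizes Gameplay Camera rigs from the character's camera properties.
; When attached to a pawn, it uses driving rigs, centering third person on the vehicle.
; Otherwise it sets shoulder side, then selects crouch, FOV, cover or Far/Balanced/Close rigs by aim state, adding a pelvis-based ragdoll offset.
; First Person on foot falls back to Close; its dedicated branch is disconnected.
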(event `self.RunCameraDirector`
  (params (DeltaTime :type "Float (single-precision)") (EvaluationContextOwner :type "Object Object Reference") (Params :type "BlueprintCameraDirectorEvaluationParams Structure (by ref)"))
  (bind _returnvalue (`self.FindEvaluationContextOwnerActor` "/Script/Engine.Actor"))
  (bind _as_sov_player_character_base (`self.As Sov Player Character Base`))
  (bind _as_sov_player_character_base_2 (`self.As Sov Player Character Base`))
  (bind _returnvalue_2 (message `/NarrativePro/Pro/Core/Character/Biped/Camera/BPI_GameplayCamera.Get_CharacterPropertiesForCamera` _returnvalue))
  (set `self.CharacterPropertiesForCamera` _returnvalue_2)
  (bind _assov_player_character_base (cast `SovPlayerCharacterBase` _returnvalue))
  (bind _output_get (set `self.As Sov Player Character Base` _assov_player_character_base))
  (set `self.AttachedToActor` (`Actor.GetAttachParentActor` _output_get))
  (set `self.ControlledPawn` (`Controller.K2_GetPawn` (`NarrativePlayerCharacter.GetPlayerController` _output_get)))
  (if (`GameplayStatics.ObjectIsA` (`self.AttachedToActor`) "/Script/Engine.Pawn")
    (`self.Mount Camera`)
    (else
      (`self.ApplyResolvedShoulderToRigs` _as_sov_player_character_base_2)
      (`self.Standard Camera`)
      (if (and (`NarrativeCharacter.IsRagdoll` _as_sov_player_character_base true) (not (`NarrativeCharacter.IsCameraInsideHead` _as_sov_player_character_base)))
        (`self.ActivateCameraRig` "/NarrativePro/Pro/Core/Character/Biped/Camera/CameraAsset_SandboxCharacter_RagdollOffset.CameraAsset_SandboxCharacter_RagdollOffset")
        (set `self.RagdollOffset` (- (- (`SceneComponent.GetSocketLocation` (`Character.Mesh` _as_sov_player_character_base_2) "pelvis") (`SceneComponent.GetSocketLocation` (`Character.Mesh` (`self.As Sov Player Character Base`)) "root")) (`KismetMathLibrary.MakeVector` 0.0 0.0 (`CapsuleComponent.GetScaledCapsuleHalfHeight` (`Character.CapsuleComponent` (`self.As Sov Player Character Base`))))))
        (`|SetCameraRigParameters` (`self.GetInitialContextResult`) (`self.RagdollOffset`))))))

(fn `ApplyResolvedShoulderToRigs`
  (params (Target :type "SovPlayerCharacterBase Object Reference"))
  (bind _returnvalue (`self.GetInitialContextResult`))
  (bind _shouldersign (`self.GetResolvedShoulderSign` Target))
  (bind _returnvalue_2 (* _shouldersign 60.0))
  (bind _returnvalue_3 (* _shouldersign 80.0))
  (bind _returnvalue_4 (`KismetMathLibrary.MakeVector` -100.0 _returnvalue_2 60.0))
  (`|SetCameraRigParameters` _returnvalue _returnvalue_4)
  (`|SetCameraRigParameters` _returnvalue _returnvalue_4)
  (`|SetCameraRigParameters` _returnvalue _returnvalue_4)
  (`|SetCameraRigParameters` _returnvalue (`KismetMathLibrary.MakeVector` -300.0 _returnvalue_3 60.0))
  (`|SetCameraRigParameters` _returnvalue (`KismetMathLibrary.MakeVector` -100.0 _returnvalue_3 60.0))
  (`|SetCameraRigParameter` _returnvalue (`KismetMathLibrary.MakeVector` -225.0 _returnvalue_2 60.0)))

(fn `GetResolvedShoulderSign`
  (params (Target :type "SovPlayerCharacterBase Object Reference"))
  (returns (ShoulderSign :type "Float (double-precision)"))
  (return (select `ESovCameraShoulder` (`.Shoulder` (break `SovCameraState` (`SovCameraControlComponent.GetCameraState` (`SovPlayerCharacterBase.GetCameraControlComponent` Target)))) :`Unchanged` 1.0 :`Right` 1.0 :`Left` -1.0)))

(fn `Mount Camera`
  (locals (PlayerOffsetFromVehicleOrigin :type "Vector Structure"))
  (bind _returnvalue (`self.GetInitialContextResult`))
  (bind (_characterpropertiesforcamera_camerastyle _characterpropertiesforcamera_cameramode _characterpropertiesforcamera_stance _characterpropertiesforcamera_isaiming _characterpropertiesforcamera_aimingfov _characterpropertiesforcamera_fov) (break `/NarrativePro/Pro/Core/Character/Biped/Camera/S_CharacterPropertiesForCamera` (`self.CharacterPropertiesForCamera`)))
  (bind _returnvalue_2 (message `/NarrativePro/Pro/Core/Character/Biped/Camera/BPI_GameplayCamera.Get_MountPropertiesForCamera` (`self.AttachedToActor`)))
  (set `self.MountPropertiesForCamera` _returnvalue_2)
  (if (`.IsAiming_17_B3146A084BD192F17087E9B30B1CD3C5` (break `/NarrativePro/Pro/Core/Character/Biped/Camera/S_CharacterPropertiesForCamera` (`self.CharacterPropertiesForCamera`)))
    (`self.ActivateCameraRig` "/NarrativePro/Pro/Core/Character/Biped/Camera/CameraAsset_SandboxCharacter_Aim_FOV.CameraAsset_SandboxCharacter_Aim_FOV")
    (`|SetCameraRigParameters` _returnvalue _characterpropertiesforcamera_aimingfov)
    (else
      (`self.ActivateCameraRig` "/NarrativePro/Pro/Core/Character/Biped/Camera/CameraAsset_SandboxCharacter_Normal_FOV.CameraAsset_SandboxCharacter_Normal_FOV")
      (`|SetCameraRigParameters` _returnvalue _characterpropertiesforcamera_fov)))
  (if (`|EnumEquality` (`.CameraStyle_9_3AB8E4E240527073591DBC8A5CC26A59` (break `/NarrativePro/Pro/Core/Character/Biped/Camera/S_CharacterPropertiesForCamera` (`self.CharacterPropertiesForCamera`))) "NewEnumerator3")
    (`self.ActivateCameraRig` "/NarrativePro/Pro/Core/Character/Biped/Camera/FirstPerson/CameraAsset_SandboxCharacter_FirstPerson_Driving.CameraAsset_SandboxCharacter_FirstPerson_Driving")
    (else
      (`self.ActivateCameraRig` "/NarrativePro/Pro/Core/Character/Biped/Camera/CameraAsset_SandboxCharacter_Driving.CameraAsset_SandboxCharacter_Driving")
      (set `local.PlayerOffsetFromVehicleOrigin` (+ (`KismetMathLibrary.InverseTransformLocation` (`Actor.GetTransform` (`self.As Sov Player Character Base`)) (`Actor.K2_GetActorLocation` (`self.ControlledPawn`))) (0.0 0.0 115.0))) ; Camera is attached to player - we need to offset so it centers around vehicle.
      (`|SetCameraRigParameters` (`self.GetInitialContextResult`) (`.VehicleCameraOffset_30_74F9455A4CA43FA216ED0F865FB18DC7` (break `/NarrativePro/Pro/Core/Character/Biped/Camera/S_MountCameraProperties` (`self.MountPropertiesForCamera`))) (`local.PlayerOffsetFromVehicleOrigin`)) ; May want offset to be config per vehicle but for now hardcode is fine
    )))

(fn `Standard Camera`
  (locals (Left :type Boolean))
  (bind _returnvalue (`self.GetInitialContextResult`))
  (bind (_characterpropertiesforcamera_camerastyle _characterpropertiesforcamera_cameramode _characterpropertiesforcamera_stance _characterpropertiesforcamera_isaiming _characterpropertiesforcamera_aimingfov _characterpropertiesforcamera_fov) (break `/NarrativePro/Pro/Core/Character/Biped/Camera/S_CharacterPropertiesForCamera` (`self.CharacterPropertiesForCamera`)))
  (bind ((`Stance_10_65A83BF64BE8EDFA2FA9FC817B1ECD53` _stance) (`IsAiming_17_B3146A084BD192F17087E9B30B1CD3C5` _isaiming)) (break `/NarrativePro/Pro/Core/Character/Biped/Camera/S_CharacterPropertiesForCamera` (`self.CharacterPropertiesForCamera`)))
  (bind _coverstate_covertransform (break `CoverState` (`NarrativeCharacterMovement.CoverState` (`NarrativeCharacter.GetNarrativeCharacterMovement` (`self.As Sov Player Character Base`)))))
  (`|ExecutionSequence`
    (:`then_1`
      ; Crouch Offset
      (switch `/NarrativePro/Pro/Core/Character/Biped/Animation/Data/E_Stance` _stance
        (:`NewEnumerator0`
          _)
        (:`NewEnumerator1`
          (`self.ActivateCameraRig` "/NarrativePro/Pro/Core/Character/Biped/Camera/CameraAsset_SandboxCharacter_Crouch_Offset.CameraAsset_SandboxCharacter_Crouch_Offset")))
      (if _isaiming
        ; Aim FOV
        (`self.ActivateCameraRig` "/NarrativePro/Pro/Core/Character/Biped/Camera/CameraAsset_SandboxCharacter_Aim_FOV.CameraAsset_SandboxCharacter_Aim_FOV")
        (`|SetCameraRigParameters` _returnvalue _characterpropertiesforcamera_aimingfov)
        (else
          (`self.ActivateCameraRig` "/NarrativePro/Pro/Core/Character/Biped/Camera/CameraAsset_SandboxCharacter_Normal_FOV.CameraAsset_SandboxCharacter_Normal_FOV")
          (`|SetCameraRigParameters` _returnvalue _characterpropertiesforcamera_fov))))
    (:`then_2`
      (if (`NarrativeCharacterMovement.HasCover` (`NarrativeCharacter.GetNarrativeCharacterMovement` (`self.As Sov Player Character Base`)))
        ; Covering
        (set `local.Left` (not (< (`KismetMathLibrary.Dot_VectorVector` (`Actor.GetActorForwardVector` (`self.As Sov Player Character Base`)) (`KismetMathLibrary.GetRightVector` (.rotation _coverstate_covertransform))) 0.0)))
        (if (`.IsAiming_17_B3146A084BD192F17087E9B30B1CD3C5` (break `/NarrativePro/Pro/Core/Character/Biped/Camera/S_CharacterPropertiesForCamera` (`self.CharacterPropertiesForCamera`)))
          (if (`self.Covered Left`)
            (`self.ActivateCameraRig` "/NarrativePro/Pro/Core/Character/Biped/Camera/Cover/CAS_Cover_Aim_R.CAS_Cover_Aim_R")
            (else
              (`self.ActivateCameraRig` "/NarrativePro/Pro/Core/Character/Biped/Camera/Cover/CAS_Cover_Aim_L.CAS_Cover_Aim_L")))
          (elif (`local.Left`)
            (`self.ActivateCameraRig` "/NarrativePro/Pro/Core/Character/Biped/Camera/Cover/CAS_Cover_Move_L.CAS_Cover_Move_L")
            (set `self.Covered Left` true)
            (else
              (`self.ActivateCameraRig` "/NarrativePro/Pro/Core/Character/Biped/Camera/Cover/CAS_Cover_Move_R.CAS_Cover_Move_R")
              (set `self.Covered Left` false))))
        (else
          (switch `/NarrativePro/Pro/Core/Character/Biped/Camera/E_CameraStyle` (`.CameraStyle_9_3AB8E4E240527073591DBC8A5CC26A59` (break `/NarrativePro/Pro/Core/Character/Biped/Camera/S_CharacterPropertiesForCamera` (`self.CharacterPropertiesForCamera`)))
            (:`NewEnumerator0`
              ; Far
              (if (`.IsAiming_17_B3146A084BD192F17087E9B30B1CD3C5` (break `/NarrativePro/Pro/Core/Character/Biped/Camera/S_CharacterPropertiesForCamera` (`self.CharacterPropertiesForCamera`)))
                (`self.ActivateCameraRig` "/Game/Aurelion/Camera/Rigs/CR_Sov_Far_Aim.CR_Sov_Far_Aim")
                (else
                  (`self.ActivateCameraRig` "/Game/Aurelion/Camera/Rigs/CR_Sov_Far_Strafe.CR_Sov_Far_Strafe"))))
            (:`NewEnumerator1`
              ; Balanced
              (if (`.IsAiming_17_B3146A084BD192F17087E9B30B1CD3C5` (break `/NarrativePro/Pro/Core/Character/Biped/Camera/S_CharacterPropertiesForCamera` (`self.CharacterPropertiesForCamera`)))
                (`self.ActivateCameraRig` "/Game/Aurelion/Camera/Rigs/CR_Sov_Balanced_Aim.CR_Sov_Balanced_Aim")
                (else
                  (`self.ActivateCameraRig` "/Game/Aurelion/Camera/Rigs/CR_Sov_Balanced_Strafe.CR_Sov_Balanced_Strafe"))))
            (:`NewEnumerator2`
              ; Close Camera
              (if (`.IsAiming_17_B3146A084BD192F17087E9B30B1CD3C5` (break `/NarrativePro/Pro/Core/Character/Biped/Camera/S_CharacterPropertiesForCamera` (`self.CharacterPropertiesForCamera`))) :!label _label
                (`self.ActivateCameraRig` "/Game/Aurelion/Camera/Rigs/CR_Sov_Close_Aim.CR_Sov_Close_Aim")
                (else
                  (`self.ActivateCameraRig` "/Game/Aurelion/Camera/Rigs/CR_Sov_Close_Strafe.CR_Sov_Close_Strafe"))))
            (:`NewEnumerator3`
              (goto _label))))))))