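; AI controller for the Aurelion contaminated drone, apparently adapted from Narrative NPC logic, handling perception, greetings and cleanup.
; Perception updates are rebroadcast to goal generators, and sighting a player character starts a looping timer for greet checks.
; GreetCheck plays greeting dialogue for nearby non-hostile players during allowed activities, unless mounted.
; CleanUp unpossesses, removing pawn (optionally delayed) and controller; damage, hearing and faction handlers are empty stubs.
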(event OnTargetPerceptionUpdated(AIPerception)
  (params (Actor :type Actor%20Object%20Reference) (Stimulus :type AI%20Stimulus%20Structure))
  (Perception|HandlePerceptionUpdate Actor Stimulus))

(event EventTick
  (params (DeltaSeconds :type Float%20%28single-precision%29)))

(event EventPossess
  (params (PossessedPawn :type Pawn%20Object%20Reference))
  ;[1 1 1] Basic init
  (bind _asnarrative_game_state (Utilities|Casting|CastToNarrativeGameState (Game|GetGameState)))
  (EventDispatchers|AssignOnFactionAttitudeChanged _asnarrative_game_state (EventDispatchers|CreateEvent :!event FactionAffiliationsChanged)))

(event EventUnPossess
  (params (UnpossessedPawn :type Pawn%20Object%20Reference))
  ;[1 1 1] Clean up controller when we unpossess, as this isn't done by default. Also allow for keeping the pawn around for required amount of time. (death uses this)
  ; Needs moved to CPP.
  (if (Variables|CleanUp|GetRequiresCleanUp)
    (if (<= (Variables|CleanUp|GetCleanUpRemovePawnDelay) 0.0)
      (Actor|DestroyActor UnpossessedPawn)
      (else
        (Actor|SetLifeSpan UnpossessedPawn (Variables|CleanUp|GetCleanUpRemovePawnDelay))))
    (Actor|SetLifeSpan 0.5)))

(event EventCleanUp
  (params (RemovePawnDelay :type Float%20%28single-precision%29))
  ;[1 1 1] Clean up controller when we unpossess, as this isn't done by default. Also allow for keeping the pawn around for required amount of time. (death uses this)
  ; Needs moved to CPP.
  (Variables|CleanUp|SetCleanUpRemovePawnDelay RemovePawnDelay)
  (Variables|CleanUp|SetRequiresCleanUp true)
  (Pawn|UnPossess))

(fn ConstructionScript)

(fn NoAggroTarget?
  (bind _blackboard (Variables|Default|GetBlackboard)
    (:then
      (Utilities|IsValid (AI|Components|Blackboard|GetValueasObject _blackboard (Variables|/Script/NarrativeArsenal.ArsenalSettings|GetBBKey_AttackTarget (Class|ArsenalStatics|GetNarrativeProSettings)))
        (:Is%20Valid
          (return false) ; We're already fighting something
        )
        (:Is%20Not%20Valid
          (return true))))
    (:else
      (return true))))

(fn OnSightSenseUpdated
  (params (Seen%20Target :type Actor%20Object%20Reference) (Successfully%20Sighted :type Boolean)))

(fn OnDamageSenseUpdated
  (params (Damager :type Actor%20Object%20Reference)))

(fn OnFactionAffiliationsChanged
  (params (Faction :type Byte :default 0) (OtherFaction :type Byte :default 0) (NewAttitude :type ETeamAttitude%20Enum :default "Friendly")))

(fn OnHearingSenseUpdated
  (params (Heard%20Target :type Actor%20Object%20Reference) (Stimulus :type AI%20Stimulus%20Structure)))

(fn HandlePerceptionUpdate
  (params (Actor :type Actor%20Object%20Reference) (Stimulus :type AI%20Stimulus%20Structure))
  (Default|CallOnPerceptionUpdated Actor Stimulus) ; Goal generators listen to this
  (bind _returnvalue (Class|AIPerceptionSystem|GetSenseClassforStimulus Stimulus))
  (if (== _returnvalue "/Script/AIModule.AISense_Sight")
    (bind _asnarrative_player_character (Utilities|Casting|CastToNarrativePlayerCharacter Actor))
    (if (Utilities|Struct|BreakAIStimulus Stimulus)
      (CallFunction|SetViewedCharacter _asnarrative_player_character)
      (else
        (CallFunction|SetViewedCharacter)))))

(fn FactionAffiliationsChanged
  (params (Faction :type Gameplay%20Tag%20Structure) (OtherFaction :type Gameplay%20Tag%20Structure) (NewAttitude :type ETeamAttitude%20Enum :default "Friendly")))

(fn SetViewedCharacter
  (params (ViewedCharacter :type Narrative%20Player%20Character%20Object%20Reference))
  (bind _output_get (Variables|Default|SetViewedCharacter ViewedCharacter))
  (Utilities|IsValid _output_get
    (:Is%20Valid
      (bind _returnvalue (Utilities|Time|SetTimerbyEvent (EventDispatchers|CreateEvent :!event GreetCheck) 2.0 true))
      (Variables|Dialogue|SetGreetCheckTimer _returnvalue))
    (:Is%20Not%20Valid
      (Utilities|Time|ClearandInvalidateTimerbyHandle (Variables|Dialogue|GetGreetCheckTimer)))))

(fn GreetCheck
  (bind _viewedcharacter (Variables|Default|GetViewedCharacter)
    (:then
      (if (< (Transformation|GetDistanceTo _viewedcharacter (Pawn|GetControlledPawn)) 3e+02)
        (if (Utilities|Array|ContainsItem (LocalVariables|GetAllowedActivities) (Utilities|GetClass (Class|NPCActivityComponent|GetCurrentActivity (Variables|Default|GetNPCActivityComponent)))) ; Only greet during certtain activities
          (LocalVariables|SetAttitude (Class|ArsenalStatics|GetAttitude self (Variables|Default|GetViewedCharacter)))
          (switch Utilities|FlowControl|Switch|SwitchonETeamAttitude (LocalVariables|GetAttitude)
            (:Friendly
              _)
            (:Neutral
              _))
          (bind _asbp_narrative_npc (Utilities|Casting|CastToBP_NarrativeNPC (Pawn|GetControlledPawn)))
          (Utilities|IsValid (Actor|GetAttachParentActor _asbp_narrative_npc) ; Bit of a catch-all for not having mounted NPCs greet - you may wish to remove this if you need that
            (:Is%20Not%20Valid
              (Class|NarrativeNPCCharacter|PlayTaggedDialogue _asbp_narrative_npc "(TagName=\"Narrative.TaggedDialogue.Greet\")" (Variables|Default|GetViewedCharacter)))))))
    (:else)))