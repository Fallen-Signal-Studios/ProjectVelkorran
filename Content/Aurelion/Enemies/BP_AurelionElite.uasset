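; Aurelion elite enemy NPC built on the Narrative framework, handling dialogue, damage, death and save identity.
; Tagged dialogue plays to nearby players after block-tag and cooldown checks; conversations can lock movement and steer head look-at.
; Damage is reported to AI, falls apply GAS damage, explosions ragdoll, and death drops a lootable physics weapon in standalone.
; Living NPCs save on destruction under unique or spawn-assigned GUIDs, and a force-holster tag stows weapons.
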(event OnDamagedby(AbilitySystemComponent)
  (params (DamagerCauserASC :type Narrative%20Ability%20System%20Component%20Object%20Reference) (Damage :type Float%20%28single-precision%29) (Spec :type Gameplay%20Effect%20Spec%20Structure%20%28by%20ref%29))
  (bind _returnvalue (Components|GetOwner DamagerCauserASC))
  (bind _returnvalue_2 (Transformation|GetActorLocation))
  (bind _returnvalue_3 (Transformation|GetActorLocation))
  (bind _asnarrative_player_state (Utilities|Casting|CastToNarrativePlayerState _returnvalue)
    (:then
      (Class|AISenseDamage|ReportDamageEvent self (PlayerState|GetPawn _asnarrative_player_state) Damage _returnvalue_2 _returnvalue_2 "None"))
    (:CastFailed
      (Class|AISenseDamage|ReportDamageEvent self _returnvalue Damage _returnvalue_3 _returnvalue_3 "None"))))

(event EventOnLanded
  (params (Hit :type Hit%20Result%20Structure%20%28by%20ref%29))
  (bind _charactermovement (Variables|Character|GetCharacterMovement))
  (bind _velocity (Variables|/Script/Engine.MovementComponent|GetVelocity _charactermovement))
  (bind _z (Math|Vector|BreakVector _velocity))
  ;[1 0.9154 0] Event On Land - Play a sound whenever the character lands similar to Event On Jumped. This logic also caches the land velocity and enables a Just Landed flag, which is used in a Chooser Table asset to select landing databases. We want this flag to be true for more than one frame, so that if movement conditions change upon landing, such as starting or stopping right after impact, landing databases will still be valid.
  (if (Class|NarrativeCharacter|IsRagdoll true)
    (if (< _z -5e+02)
      (CallFunction|PlayAudioEvent "(TagName=\"Foley.Event.Tumble\")" (Math|Float|MapRangeClamped _z -5e+02 -9e+02 0.5 1.5) 1.0))
    (else
      (CallFunction|PlayAudioEvent "(TagName=\"Foley.Event.Land\")" (Math|Float|MapRangeClamped (.z (Variables|Default|GetLandVelocity)) -5e+02 -9e+02 0.5 1.5) 1.0))))

(event EventBeginPlay
  (|CallParentFunction)
  ;[0.15 0.15 0.15 0.5] Interim fix for NPR-183 - needs folded into ability
  (Networking|SwitchHasAuthority
    (:Authority
      (bind _tagcount (Ability|Tasks|WaitGameplayTagCountChangedOnActor 0 "(TagName=\"Narrative.State.Weapon.ForceHolster\")")
        (:TagCountChanged
          (if (<= _tagcount 0)
            (Class|NarrativeCharacter|SetWieldState (Variables|Default|GetStowedWeapon))
            (Variables|Default|SetStowedWeapon "")
            (elif (> (Utilities|Array|Length (GameplayTags|BreakGameplayTagContainer (.EquipSlots (Utilities|Struct|BreakWeaponWieldState (Variables|Default|GetWieldState))))) 0) ; Stow our wield, provided we actually have one
              (Variables|Default|SetStowedWeapon (Variables|Default|GetWieldState))
              (Class|NarrativeCharacter|SetWieldState (Utilities|Struct|MakeWeaponWieldState "(GameplayTags=)" 0 "(GameplayTags=)")))))))))

(event EventHandleExplosionImpact
  (params (ExplosionCauser :type Narrative%20Ability%20System%20Component%20Object%20Reference) (ExplosionLocation :type Vector%20%28by%20ref%29 :default "0, 0, 0") (IntendedDamage :type Float%20%28single-precision%29))
  (Class|NarrativeCharacter|RagdollwithDamageandImpulse 3.0 (* (Math|Vector|Normalize (- (Transformation|GetActorLocation) ExplosionLocation)) 5e+03) 0.0))

(event EventHandleDeath
  (params (KilledActor :type Actor%20Object%20Reference) (KilledActorASC :type Narrative%20Ability%20System%20Component%20Object%20Reference) (bIsDead :type Boolean))
  ;[0.15 0.15 0.15 0.5] Just a neat bit of polish - make the enemy drop their weapon and turn it into a physics actor - it will still be destroyed once you loot it from the enemy
  (|CallParentFunction KilledActor KilledActorASC bIsDead)
  (Class|NPCActivityComponent|RemoveAllGoals (Class|NarrativeNPCCharacter|GetActivityComponent))
  (bind _asbp_weapon_visual_base (Utilities|Casting|CastToBP_WeaponVisualBase (Class|NarrativeCharacter|GetEquippedWeaponVisual)))
  (if (Class|KismetSystemLibrary|IsStandalone)
    (Transformation|DetachFromActor _asbp_weapon_visual_base "KeepWorld" "KeepWorld" "KeepWorld")
    (Physics|SetSimulatePhysics (Variables|/Script/NarrativeArsenal.WeaponVisual|GetWeaponMesh _asbp_weapon_visual_base) true)
    (Collision|SetCollisionResponsetoChannel (Variables|/Script/NarrativeArsenal.WeaponVisual|GetWeaponMesh _asbp_weapon_visual_base) "ECC_Pawn" "ECR_Ignore")
    (Collision|SetCollisionResponsetoChannel (Variables|/Script/NarrativeArsenal.WeaponVisual|GetWeaponMesh _asbp_weapon_visual_base) "ECC_WorldStatic" "ECR_Block")
    (Collision|SetCollisionResponsetoChannel (Variables|/Script/NarrativeArsenal.WeaponVisual|GetWeaponMesh _asbp_weapon_visual_base) "ECC_GameTraceChannel1" "ECR_Block")
    ;[0.15 0.15 0.15 0.5] add dropped weapon pickup component for player to pick up this weapon
    (Collision|SetCollisionEnabled (Variables|/Script/NarrativeArsenal.WeaponVisual|GetWeaponMesh _asbp_weapon_visual_base) "QueryAndPhysics")
    (bind _returnvalue (Game|AddComponentbyClass _asbp_weapon_visual_base "/NarrativePro/Pro/Core/BP/World/Interactable_DroppedWeapon.Interactable_DroppedWeapon_C"))
    (Default|SetWeaponItemforPickup _returnvalue (Utilities|GetClass (Class|NarrativeCharacter|GetWeapon true)))
    (else
      (Actor|DestroyActor _asbp_weapon_visual_base))))

(event EventExecutePlayTaggedDialogue
  (params (Dialogue :type Tagged%20Dialogue%20Structure) (DialogueInstigator :type Actor%20Object%20Reference))
  (bind (_tag _dialogue) (Utilities|Struct|BreakTaggedDialogue Dialogue))
  ;[1 1 1] Play a local dialogue via a tag, like greet, taunt, etc
  (bind (_can_play _playon) (Narrative|CheckCanPlayTaggedDialogue Dialogue))
  (if _can_play
    (bind _class (Utilities|AsyncLoadClassAsset _dialogue)
      (:Completed
        (bind _asdialogue (Utilities|Casting|CastToDialogueClass _class))
        (for _array_element _playon
          (Class|TalesComponent|BeginDialogue (Class|NarrativeFunctionLibrary|GetTalesComponentfromTarget _array_element) _asdialogue (Utilities|Struct|MakeDialoguePlayParams "None" 10 true false true false (Utilities|Array|MakeArray self))) ; TODO this might need to be Soft Reffed dialogue as when client replicates it may hitch from dialogue asset load
          (Utilities|Map|Add (Variables|/Script/NarrativeArsenal.TalesComponent|GetTaggedDialogueLastPlayTimes (Class|NarrativeFunctionLibrary|GetTalesComponentfromTarget _array_element)) _tag (Utilities|Time|GetTimeSeconds)))))))

(event EventOnEnterDialogue
  (params (Dialogue :type Dialogue%20Object%20Reference))
  ;[1 1 1] Lock NPCs movement if they are talking - this way even if the NPC starts a new goal or something they should stay in place until dialogue is over.
  (if (not (Variables|/Script/NarrativeArsenal.Dialogue|GetbFreeMovement Dialogue))
    (Ability|GameplayEffect|AddLooseGameplayTags self (GameplayTags|MakeLiteralGameplayTagContainer "(GameplayTags=((TagName=\"Narrative.State.Movement.Lock\")))"))))

(event EventOnEndDialogue
  (params (Dialogue :type Dialogue%20Object%20Reference))
  ;[1 1 1] Lock NPCs movement if they are talking - this way even if the NPC starts a new goal or something they should stay in place until dialogue is over.
  (if (not (Variables|/Script/NarrativeArsenal.Dialogue|GetbFreeMovement Dialogue))
    (Ability|GameplayEffect|RemoveLooseGameplayTags self (GameplayTags|MakeLiteralGameplayTagContainer "(GameplayTags=((TagName=\"Narrative.State.Movement.Lock\")))"))))

(event EventDestroyed
  (bind _returnvalue (Subsystems|GetNarrativeSaveSubsystem))
  (bind _self self)
  ;[1 1 1] When an NPC is destroyed, provided they weren't dead they must have been unloaded by WP or some other means. We'll create a save record for them so when they spawn in again they have their data!
  (if (GameplayTags|HasMatchingGameplayTag (Variables|Default|GetAbilitySystemComponent) "(TagName=\"Narrative.State.IsDead\")")
    (Class|NarrativeSaveSubsystem|RemoveSingleActor _returnvalue _self) ; We're dead and no longer require a save record.
    (else
      (Class|NarrativeSaveSubsystem|SaveSingleActor _returnvalue _self) ; We were destroyed for some other reason whilst alive and require a save record
    )))

(fn ConstructionScript)

(fn GetHeadLookatLocation
  (bind _returnvalue (Class|NarrativeFunctionLibrary|GetTalesComponent))
  (Utilities|IsValid _returnvalue
    (:Is%20Valid
      (LocalVariables|SetCurrentDialogue (Variables|/Script/NarrativeArsenal.TalesComponent|GetCurrentDialogue _returnvalue))
      (LocalVariables|GetCurrentDialogue
        (:then
          ;[1 1 1] If in dialogue look at speaker if listening or at listener if speaking
          (bind _output_get (LocalVariables|SetAvatarToLookAt (select (== (Variables|/Script/NarrativeArsenal.Dialogue|GetCurrentSpeakerAvatar (LocalVariables|GetCurrentDialogue)) self) (Variables|/Script/NarrativeArsenal.Dialogue|GetCurrentListenerAvatar (LocalVariables|GetCurrentDialogue)) (Variables|/Script/NarrativeArsenal.Dialogue|GetCurrentSpeakerAvatar (LocalVariables|GetCurrentDialogue)))))
          (Utilities|IsValid _output_get
            (:Is%20Valid
              (if (< (Transformation|GetDistanceTo (LocalVariables|GetAvatarToLookAt) self) 2e+03)
                (return true (Class|Dialogue|GetSpeakerHeadLocation (LocalVariables|GetCurrentDialogue) (LocalVariables|GetAvatarToLookAt)))
                (else
                  _)))
            (:Is%20Not%20Valid
              (return false "0, 0, 0"))))
        (:else
          ;[1 1 1] If we're not in dialogue, look at the player if we are nearby
          (bind _lookatchartarget (Variables|Default|GetLookAtCharTarget)
            (:then
              ;[0.15 0.15 0.15 0.5] Allows sequencer to override what character we look at
              (return true (Transformation|GetSocketLocation (Variables|/Script/Engine.Character|GetMesh _lookatchartarget) "head")))
            (:else
              (if (GameplayTags|HasMatchingGameplayTag "(TagName=\"Narrative.State.NPC.DisableLookAtNearbyChar\")")
                _
                (else
                  (bind _asbp_narrative_npccontroller (Utilities|Casting|CastToBP_NarrativeNPCController (AI|GetAIController self)))
                  (bind _viewedcharacter (Variables|/NarrativePro/Pro/Core/AI/BP/BP_NarrativeNPCController.BP_NarrativeNPCController_C|GetViewedCharacter _asbp_narrative_npccontroller)
                    (:then
                      (return true (Transformation|GetSocketLocation (Variables|/Script/Engine.Character|GetMesh _viewedcharacter) "head")))
                    (:else
                      _))))))))
      (return false "0, 0, 0"))))

(fn GetActorGUID
  (bind _spawninfo (Variables|Default|GetSpawnInfo))
  (bind _spawnassignedsaveguid (Utilities|Struct|BreakNPCSpawnInfo _spawninfo))
  (Utilities|IsValid (Variables|Default|GetNPCDefinition)
    (:Is%20Valid
      (if (Variables|/Script/NarrativeArsenal.NPCDefinition|GetbAllowMultipleInstances (Variables|Default|GetNPCDefinition))
        ;[1 1 1] Non-unique NPCs use a save GUID their spawn assigns them, so that way if you come back to a spawn its NPC will have the same data.
        (return _spawnassignedsaveguid) ; Non-unique NPCs use a GUID generated by the actor instance, because we need to make multiple records for each of the NPCs.
        (else
          (return (Variables|/Script/NarrativeArsenal.NPCDefinition|GetUniqueNPCGUID (Variables|Default|GetNPCDefinition))) ; Unique NPCs use a GUID defined in the NPC Data Asset. This ensures unique NPCs only ever get 1 record created, which makes sense because they are unique!\nThis GUID can also be empty, which means the save system skips over this NPC - useful for transient NPCs
        )))
    (:Is%20Not%20Valid
      (return _spawnassignedsaveguid))))

(fn ShouldRespawn
  (return false) ; NPCs should never be respawned by the save system - their owning settlement or the player they are following will handle spawning them back in
)

(fn HandleFallDamage
  (params (Fall%20Hit :type Hit%20Result%20Structure))
  (bind _self self)
  (bind _charactermovement (Variables|Character|GetCharacterMovement))
  (bind _returnvalue (Ability|GetAbilitySystemComponent _self))
  (bind _velocity (Variables|/Script/Engine.MovementComponent|GetVelocity _charactermovement))
  (bind _returnvalue_2 (Ability|Attribute|GetFloatAttributefromAbilitySystemComponent _returnvalue "(AttributeName=\"MaxHealth\",Attribute=/Script/NarrativeArsenal.NarrativeAttributeSetBase:MaxHealth,AttributeOwner=\"/Script/CoreUObject.Class'/Script/NarrativeArsenal.NarrativeAttributeSetBase'\")"))
  (bind _z (Math|Vector|BreakVector _velocity))
  (bind _returnvalue_3 (Math|Float|MapRangeClamped _z -1.3e+03 -1.8e+03 0.0 _returnvalue_2))
  (if (> (Actor|GetGameTimeSinceCreation) 7.0) ; On start sometimes we get high fall damage values
    (bind _output_get (LocalVariables|SetFallDamageVal _returnvalue_3))
    (if (> _output_get 0.1)
      (bind _returnvalue_4 (Ability|GameplayEffect|AssignTagSetbyCallerMagnitude (GameplayEffects|MakeOutgoingSpec _returnvalue "/NarrativePro/Pro/Core/Abilities/GameplayEffects/GE_Damage_SetByCaller.GE_Damage_SetByCaller_C" 1.0 (GameplayEffects|MakeEffectContext _returnvalue)) "(TagName=\"SetByCaller.Damage\")" _returnvalue_3))
      (GameplayEffects|ApplyGameplayEffectSpecToSelf _returnvalue _returnvalue_4))))

(fn CheckCanPlayTaggedDialogue
  (params (TaggedDialogue :type Tagged%20Dialogue%20Structure%20%28by%20ref%29))
  (if (> (Actor|GetGameTimeSinceCreation) 1.0)
    (if (Class|NarrativeCharacter|IsAlive)
      (bind _outactors (Collision|SphereOverlapActors (Transformation|GetActorLocation) (.MaxDistance (Utilities|Struct|BreakTaggedDialogue TaggedDialogue)) (Utilities|Array|MakeArray "ObjectTypeQuery3") "/NarrativePro/Pro/Core/Character/BP/BP_NarrativePlayerCharacter_TarrikBase.BP_NarrativePlayerCharacter_TarrikBase_C" (Utilities|Array|MakeArray self))) ; not working, not sure why
      (LocalVariables|SetPlayersToCheck _outactors)
      (if (<= (Utilities|Array|Length (LocalVariables|GetPlayersToCheck)) 0)
        (Development|PrintString (Utilities|String|Append "failed taggged dialogue as " (GameplayTags|GetDebugStringfromGameplayTag (.tag TaggedDialogue)) " played but no listeners were within " (Utilities|String|ToString(Float) (.maxdistance TaggedDialogue)) "units of dist") false false)
        (return false 0) ; no one is around to hear the dialogue
        (else
          (LocalVariables|SetAllListenersWantDialogue true)
          (for _array_element (LocalVariables|GetPlayersToCheck)
            (bind _asnarrative_player_character (Utilities|Casting|CastToNarrativePlayerCharacter _array_element))
            (if (GameplayTags|HasAnyMatchingGameplayTags _asnarrative_player_character (LocalVariables|GetBlockTaggedDialogueTags))
              (return false 0)
              (else
                (LocalVariables|SetTalesComp (Class|NarrativeFunctionLibrary|GetTalesComponentfromTarget _asnarrative_player_character))
                (Utilities|IsValid (LocalVariables|GetTalesComp)
                  (:Is%20Valid
                    (if (Class|TalesComponent|IsinDialogue (LocalVariables|GetTalesComp)) ; Tagged dialogue is low priority and shouldnt interrupt existing dialogue
                      (return false 0)
                      (elif (.ReturnValue (Utilities|Map|Find (Variables|/Script/NarrativeArsenal.TalesComponent|GetTaggedDialogueLastPlayTimes (LocalVariables|GetTalesComp)) (.tag TaggedDialogue)))
                        (if (> (- (Utilities|Time|GetTimeSeconds) (.Value (Utilities|Map|Find (Variables|/Script/NarrativeArsenal.TalesComponent|GetTaggedDialogueLastPlayTimes (LocalVariables|GetTalesComp)) (.tag TaggedDialogue)))) (Math|Float|SelectFloat (.Value (Utilities|Map|Find (Variables|/Script/NarrativeArsenal.TalesComponent|GetTaggedDialogueCooldowns (LocalVariables|GetTalesComp)) (.Tag (Utilities|Struct|BreakTaggedDialogue TaggedDialogue)))) (Variables|/Script/NarrativeArsenal.TalesComponent|GetFallbackCooldown (LocalVariables|GetTalesComp)) (.ReturnValue (Utilities|Map|Find (Variables|/Script/NarrativeArsenal.TalesComponent|GetTaggedDialogueCooldowns (LocalVariables|GetTalesComp)) (.Tag (Utilities|Struct|BreakTaggedDialogue TaggedDialogue))))))
                          (return true (LocalVariables|GetPlayersToCheck))
                          (else
                            (Development|PrintString (Utilities|String|Append "failed taggged dialogue as " (GameplayTags|GetDebugStringfromGameplayTag (.tag TaggedDialogue)) " played " (Utilities|String|ToString(Float) (- (Utilities|Time|GetTimeSeconds) (.Value (Utilities|Map|Find (Variables|/Script/NarrativeArsenal.TalesComponent|GetTaggedDialogueLastPlayTimes (LocalVariables|GetTalesComp)) (.tag TaggedDialogue))))) " seconds ago and cooldown is " (Utilities|String|ToString(Float) (Math|Float|SelectFloat (.Value (Utilities|Map|Find (Variables|/Script/NarrativeArsenal.TalesComponent|GetTaggedDialogueCooldowns (LocalVariables|GetTalesComp)) (.Tag (Utilities|Struct|BreakTaggedDialogue TaggedDialogue)))) (Variables|/Script/NarrativeArsenal.TalesComponent|GetFallbackCooldown (LocalVariables|GetTalesComp)) (.ReturnValue (Utilities|Map|Find (Variables|/Script/NarrativeArsenal.TalesComponent|GetTaggedDialogueCooldowns (LocalVariables|GetTalesComp)) (.Tag (Utilities|Struct|BreakTaggedDialogue TaggedDialogue))))))) false false)
                            (return false 0))))))
                  (:Is%20Not%20Valid
                    (return false 0))))))
          (return true (LocalVariables|GetPlayersToCheck))))
      (else
        _)))
  (return false 0))

(fn PlayAudioEvent
  (params (Value :type Gameplay%20Tag%20Structure) (VolumeMultiplier :type Float%20%28single-precision%29) (PitchMultiplier :type Float%20%28single-precision%29))
  (bind _foleyaudiobank (CallFunction|GetFoleyAudioBank))
  (Audio|PlaySoundatLocation (.Value (Utilities|Map|Find (.FoleySounds (Utilities|Struct|BreakNarrativeFoleySound (.Value (Utilities|Map|Find (Variables|/Script/NarrativeArsenal.FoleyAudioBank|GetFoleySounds _foleyaudiobank) Value)))) "SurfaceType_Default")) (Transformation|GetWorldLocation (Variables|Character|GetMesh)) "0, 0, 0" VolumeMultiplier PitchMultiplier 0.0 0 0 0 0))

(fn CalcSightStrength
  (params (Start :type Vector%20%28by%20ref%29 :default "0, 0, 0") (End :type Vector%20%28by%20ref%29 :default "0, 0, 0") (Looker :type Actor%20Object%20Reference))
  (return 1e+01))

(fn CanPlayFootstepSounds
  (return false) ; NPCs dont need to play these, as they get spammy
)

(fn GetFoleyAudioBank
  (return "/NarrativePro/Pro/Core/Audio/Foley/DA_DefaultNarrativeFoley.DA_DefaultNarrativeFoley"))